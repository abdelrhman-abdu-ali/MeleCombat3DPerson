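; Survival game mode Blueprint that announces wave progress on screen as the survival state changes.
; On BeginPlay it binds to the state-change event and switches on the state, feeding two helpers that create wave text widgets, with or without a countdown.
; The final wave also sets the enemy spawn delay and shows a delayed "LastWave" banner.
; All-waves-done and player-death states only print debug strings.
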(event Custom|OnSurvialGameModeStateChanged_Event
  (params (CurrentState :type EWarriorSurvialGameModeState%20Enum :default "WaitSpawnNewWave"))
  (switch Utilities|FlowControl|Switch|SwitchonEWarriorSurvialGameModeState CurrentState
    (:WaitSpawnNewWave
      (CallFunction|CreatWaveWidgetwithCountDown "New Wave Coming In !!" (Variables|Default|GetSpawnNewWaveWaitTime)))
    (:SpawningNewWave
      (CallFunction|CreatWaveWidgetNoCountDown (Utilities|Text|FormatText "Wave{CurrentWaveCount} " (Variables|Default|GetCurrentWaveCount)))
      (if (== (Variables|Default|GetTotalWavesToSpawn) (Variables|Default|GetCurrentWaveCount))
        (Variables|Default|SetSpawnEnemiesDelayTime 4.0)
        (Utilities|FlowControl|Delay 2.0)
        (CallFunction|CreatWaveWidgetNoCountDown "LastWave")))
    (:WaveCompleted
      (CallFunction|CreatWaveWidgetwithCountDown (Utilities|Text|FormatText "Wave{CurrentWaveCount} Completed" (Variables|Default|GetCurrentWaveCount)) (Variables|Default|GetWaveCompletedWaitTime)))
    (:AllWavesDone
      (Development|PrintString "AllWavesDone" true true "(R=0.098612,G=1.000000,B=0.154049,A=1.000000)"))
    (:PlayerDied
      (Development|PrintString "playerDied" true true "(R=1.000000,G=0.080261,B=0.280946,A=1.000000)"))))

(event EventBeginPlay
  (EventDispatchers|AssignOnSurvialGameModeStateChanged (delegate Custom|OnSurvialGameModeStateChanged_Event)))

(event EventTick
  (params (DeltaSeconds :type Float%20%28single-precision%29)))

(fn ConstructionScript)

(fn CreatWaveWidgetwithCountDown
  (params (TextContentToDisplay :type Text) (inTotalCountDownTime :type Float%20%28double-precision%29))
  (bind _returnvalue (UserInterface|CreateWidget "/Game/Widgets/GameModeWidgets/WBP_waveTextWithCountDown.WBP_waveTextWithCountDown_C"))
  (UserInterface|Viewport|AddtoViewport _returnvalue 0)
  (Rendering|Components|TextRender|SetText (Variables|/Game/Widgets/GameModeWidgets/WBP_waveTextWithCountDown.WBP_waveTextWithCountDown_C|GetTextBlock-WaveText _returnvalue) TextContentToDisplay)
  (Default|StartCountDown _returnvalue inTotalCountDownTime))

(fn CreatWaveWidgetNoCountDown
  (params (TextContentToDisplay :type Text))
  (bind _returnvalue (UserInterface|CreateWidget "/Game/Widgets/GameModeWidgets/WBP_waveText.WBP_waveText_C"))
  (UserInterface|Viewport|AddtoViewport _returnvalue 0)
  (Rendering|Components|TextRender|SetText (Variables|/Game/Widgets/GameModeWidgets/WBP_waveText.WBP_waveText_C|GetTextBlock-WaveText _returnvalue) TextContentToDisplay))