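; Base projectile Blueprint that handles the sound and visual effects of a projectile's spawn and impact.
; On BeginPlay it plays a spawn sound, attaches a flight sound that stops with the projectile, and spawns a forward-facing Niagara muzzle effect.
; The OnSpawnProjectileHitFX event plays the impact sound and effect at the supplied hit location.
; Every asset is a validity-checked variable, and the graph contains no movement or damage logic.
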(event EventBeginPlay
  (Utilities|FlowControl|Sequence
    (:then_0
      (bind _projectilespawnedsound (Variables|Default|GetProjectileSpawnedSound)
        (:then
          (Audio|PlaySoundatLocation _projectilespawnedsound (Transformation|GetActorLocation) "0, 0, 0" 1.0 1.0 0.0 0 0 0 0))
        (:else)))
    (:then_1
      (bind _projectileflysound (Variables|Default|GetProjectileFlySound)
        (:then
          (Audio|SpawnSoundAttached _projectileflysound (Variables|Transformation|GetRootComponent) "None" "0, 0, 0" "0, 0, 0" "KeepRelativeOffset" true 1.0 1.0 0.0 0 0))
        (:else)))
    (:then_2
      (bind _projectilemuzzlfx (Variables|Default|GetProjectileMuzzlFX)
        (:then
          (Niagara|SpawnSystematLocation _projectilemuzzlfx (Transformation|GetActorLocation) (Math|Conversions|RotationFromXVector (Transformation|GetActorForwardVector))))
        (:else)))))

(event EventOnSpawnProjectileHitFX
  (params (HitLocation :type Vector%20%28by%20ref%29 :default "0, 0, 0"))
  (Utilities|FlowControl|Sequence
    (:then_0
      (bind _projectileimpactsound (Variables|Default|GetProjectileImpactSound)
        (:then
          (Audio|PlaySoundatLocation _projectileimpactsound HitLocation "0, 0, 0" 1.0 1.0 0.0 0 0 0 0))
        (:else)))
    (:then_1
      (bind _projectileimpateffects (Variables|Default|GetProjectileImpatEffects)
        (:then
          (Niagara|SpawnSystematLocation _projectileimpateffects HitLocation))
        (:else)))))

(fn ConstructionScript)